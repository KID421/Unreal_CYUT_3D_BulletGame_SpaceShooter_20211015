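; BP_敵機 is an enemy aircraft that moves steadily along world negative Z and fires bullets at a regular interval.
; Tick offsets its location by the movement speed each frame, without sweeping or delta-time scaling.
; A looping timer from BeginPlay spawns BP_子彈 at the 生成子彈位置 component, passing speed, size, direction and an enemy emissive material.
; The construction script only assigns the movement speed to itself.
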(event Custom|生成子彈
  ;[0.4922 0.1218 0.1218] 發射子彈
  (Game|SpawnActorfromClass "/Game/BP/BP_子彈.BP_子彈_C" (Transformation|GetWorldTransform (Variables|Default|Get生成子彈位置)) "Undefined" 0 (Variables|子彈資訊|Get子彈速度) (Variables|子彈資訊|Get子彈尺寸) (Variables|子彈資訊|Get子彈飛行方向) "/Game/材質球/M_自發光_敵機.M_自發光_敵機" 0))

(event EventTick
  (params (DeltaSeconds :type Float%20%28single-precision%29))
  ;[0.4922 0.1218 0.1218] 移動
  (Transformation|SetActorLocation (- (Transformation|GetActorLocation) (Math|Vector|MakeVector 0.0 0.0 (Variables|Default|Get移動速度))) false false))

(event EventBeginPlay
  ;[0.4922 0.1218 0.1218] 發射子彈
  (Utilities|Time|SetTimerbyFunctionName 0 "生成子彈" (Variables|Default|Get發射間隔) true))

(fn ConstructionScript
  (Variables|Default|Set移動速度 (Variables|Default|Get移動速度)))