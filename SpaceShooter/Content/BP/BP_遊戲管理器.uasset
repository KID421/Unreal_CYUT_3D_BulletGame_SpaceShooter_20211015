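; BP_遊戲管理器 is a game manager Blueprint that lets the player restart or quit once the game is over.
; On BeginPlay it caches the game mode as BP_遊戲模式.
; The restart and quit input actions check that game mode's game-over flag (是否遊戲結束), then either reload the 遊戲地圖 level or quit the game.
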(event EventBeginPlay
  ;[0.4922 0.1218 0.1218] 取得遊戲模式
  (bind _asbp_遊戲模式 (Utilities|Casting|CastToBP_遊戲模式 (Game|GetGameMode)))
  (Variables|Default|SetBP%20遊戲模式 _asbp_遊戲模式))

(event Input|ActionEvents|InputAction重新遊戲
  (params (Key :type Key%20Structure :default "None"))
  ;[0.09541 0.1452 0.4453] 重新與離開遊戲
  (:Pressed
    (if (Variables|/Game/BP/BP_遊戲模式.BP_遊戲模式_C|Get是否遊戲結束 (Variables|Default|GetBP%20遊戲模式))
      (Game|OpenLevel(byName) "遊戲地圖") ; 開啟地圖
    )))

(event Input|ActionEvents|InputAction離開遊戲
  (params (Key :type Key%20Structure :default "None"))
  ;[0.09541 0.1452 0.4453] 重新與離開遊戲
  (:Pressed
    (if (Variables|/Game/BP/BP_遊戲模式.BP_遊戲模式_C|Get是否遊戲結束 (Variables|Default|GetBP%20遊戲模式))
      (Game|QuitGame 0 "Quit" false) ; 離開遊戲
    )))

(fn ConstructionScript)