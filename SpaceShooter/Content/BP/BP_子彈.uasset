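; BP_子彈 is a bullet projectile Blueprint built from a sphere (球體) and a projectile movement component.
; Its construction script applies the size, speed, flight direction and material variables, using the speed as both initial and maximum speed.
; NewFunction0 repeats that setup from passed-in values, without setting the material.
; The event graph holds only disabled placeholder events, so it adds no hit or overlap logic.
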(event EventBeginPlay)

(event Collision|EventActorBeginOverlap
  (params (OtherActor :type Actor%20Object%20Reference)))

(event EventTick
  (params (DeltaSeconds :type Float%20%28single-precision%29)))

(fn ConstructionScript
  (bind _投射物移動元件 (Variables|Default|Get投射物移動元件))
  (Transformation|SetWorldScale3D (Variables|Default|Get球體) (* "1.000000,1.000000,1.000000" (Variables|Default|Get子彈尺寸))) ; 設定世界尺寸
  (bind _output_get (Variables|/Script/Engine.ProjectileMovementComponent|SetMaxSpeed _投射物移動元件 (Variables|Default|Get子彈速度))) ; 設定最大速度
  (Variables|/Script/Engine.ProjectileMovementComponent|SetInitialSpeed _投射物移動元件 _output_get) ; 設定初始速度
  (Variables|/Script/Engine.MovementComponent|SetVelocity _投射物移動元件 (Variables|Default|Get子彈飛行方向)) ; 設定加速度 (方向)
  (Rendering|Material|SetMaterial (Variables|Default|Get球體) 0 (Variables|Default|Get子彈材質)) ; 設定材質球
)

(fn NewFunction0
  (params (Velocity :type Vector) (MaxSpeed :type Float%20%28single-precision%29) (B :type Float%20%28single-precision%29))
  (bind _投射物移動元件 (Variables|Default|Get投射物移動元件))
  (Transformation|SetWorldScale3D (Variables|Default|Get球體) (* "1.000000,1.000000,1.000000" B)) ; 設定世界尺寸
  (bind _output_get (Variables|/Script/Engine.ProjectileMovementComponent|SetMaxSpeed _投射物移動元件 MaxSpeed)) ; 設定最大速度
  (Variables|/Script/Engine.ProjectileMovementComponent|SetInitialSpeed _投射物移動元件 _output_get) ; 設定初始速度
  (Variables|/Script/Engine.MovementComponent|SetVelocity _投射物移動元件 Velocity) ; 設定加速度 (方向)
)