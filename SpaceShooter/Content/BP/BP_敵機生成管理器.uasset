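; Enemy plane spawn manager actor that continuously spawns BP_敵機 enemy planes during play.
; On BeginPlay it calls the 生成敵機 event, which spawns a plane at a random X between left and right bounds on a set Z, with fixed rotation, configurable scale and random move speed.
; The event then waits a random interval and calls itself again, forming an endless spawn loop.
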(event Custom|生成敵機
  ;[0.4922 0.1218 0.1218] 生成敵機
  (Game|SpawnActorfromClass "/Game/BP/BP_敵機.BP_敵機_C" (Math|Transform|MakeTransform (Math|Vector|MakeVector (Math|Random|RandomFloatinRange (Variables|Default|Get座標左邊界) (Variables|Default|Get座標右邊界)) 0.0 (Variables|Default|Get座標Z軸)) "0, 0,90.000000" (* "1.000000,1.000000,1.000000" (Variables|Default|Get敵機尺寸))) "Undefined" 0 (Math|Random|RandomFloatinRange (Variables|Default|Get敵機最小速度) (Variables|Default|Get敵機最大速度)) 0)
  (Utilities|FlowControl|Delay (Math|Random|RandomFloatinRange (Variables|Default|Get生成最小間隔) (Variables|Default|Get生成最大間隔))) ; 延遲：等待指定秒數後再執行後方節點
  (CallFunction|生成敵機))

(event EventBeginPlay
  ;[0.4922 0.1218 0.1218] 生成敵機
  (CallFunction|生成敵機))

(fn ConstructionScript)