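; Player spaceship Blueprint that flies into the scene on start, then moves in the X/Z plane under axis input.
; On BeginPlay, if the game mode cast succeeds, a timeline lerps position and yaw through the entrance, then enables control.
; A shared function smooths the horizontal and vertical axis speeds with FInterpTo.
; Tick applies those speeds within clamped bounds and interpolates yaw from horizontal speed to turn the ship.
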(event EventTick
  (params (DeltaSeconds :type Float%20%28single-precision%29))
  (bind _returnvalue (Transformation|GetActorLocation))
  (bind _運算後速度水平 (Variables|Default|Get運算後速度水平))
  (bind _運算後速度垂直 (Variables|Default|Get運算後速度垂直))
  (bind _returnvalue_2 (+ _returnvalue (Math|Vector|MakeVector _運算後速度水平 0.0 _運算後速度垂直)))
  ;[0.4922 0.1218 0.1218] 持續執行：移動與旋轉
  (Variables|Default|Set一幀時間 DeltaSeconds)
  (if (Variables|Default|Get開關控制) ; 分支：判斷式，當布林值勾選會從 True 出去
    (Transformation|SetActorLocation (Math|Vector|MakeVector (Math|Float|Clamp(Float) (.x _returnvalue_2) (Variables|Default|Get水平左邊界) (Variables|Default|Get水平右邊界)) 0.0 (Math|Float|Clamp(Float) (.z _returnvalue_2) (Variables|Default|Get垂直下邊界) (Variables|Default|Get垂直上邊界))) false false)
    (Transformation|SetActorRotation (Math|Interpolation|RInterpTo "0, 0, 0" (Math|Rotator|MakeRotator 0.0 0.0 (* (Variables|Default|Get運算後速度水平) (Variables|Default|Get旋轉速度))) (Variables|Default|Get一幀時間) (Variables|Default|Get平滑旋轉速度)))))

(event EventBeginPlay
  ;[0.4922 0.1218 0.1218] 登場效果
  (Utilities|Casting|CastToBP_遊戲模式 (Game|GetGameMode))
  (Variables|Default|Set初始位置 (Transformation|GetActorLocation)) ; 設定變數：變更變數的值
  (Variables|Default|Set初始角度 (.Yaw (Math|Rotator|BreakRotator (Transformation|GetActorRotation)))) ; 設定變數：綠色為浮點數
  (bind _登場時間值 (Timeline|登場時間軸 Play) ; 時間軸：可自行設定時間以及輸出的值
    (:Update
      (Transformation|SetActorLocation (Math|Vector|Lerp(Vector) (Variables|Default|Get初始位置) (+ (Variables|Default|Get初始位置) (Variables|Default|Get前進位置)) _登場時間值) false false) ; 設定物件座標
      (Transformation|SetActorRotation (Math|Rotator|Lerp(Rotator) (Math|Rotator|MakeRotator 0.0 0.0 (Variables|Default|Get初始角度)) (Math|Rotator|MakeRotator 0.0 0.0 (Variables|Default|Get前進角度)) _登場時間值)) ; 設定物件角度
    )
    (:Finished
      (Variables|Default|Set開關控制 true))))

(event Input|AxisEvents|InputAxis水平
  (params (AxisValue :type Float%20%28single-precision%29))
  ;[0.09541 0.1452 0.4453] 水平與垂直移動
  (bind _運算後速度 (CallFunction|處理平滑速度 AxisValue (Variables|Default|Get速度水平) (Variables|Default|Get運算後速度水平)))
  (Variables|Default|Set運算後速度水平 _運算後速度))

(event Input|AxisEvents|InputAxis垂直
  (params (AxisValue :type Float%20%28single-precision%29))
  ;[0.09541 0.1452 0.4453] 水平與垂直移動
  (bind _運算後速度 (CallFunction|處理平滑速度 AxisValue (Variables|Default|Get速度垂直) (Variables|Default|Get運算後速度垂直)))
  (Variables|Default|Set運算後速度垂直 _運算後速度))

(fn ConstructionScript)

(fn 處理平滑速度
  (params (軸向值 :type Float%20%28single-precision%29) (速度 :type Float%20%28single-precision%29) (運算前速度 :type Float%20%28single-precision%29))
  (return (Math|Interpolation|FInterpTo 運算前速度 (* 軸向值 速度) (Variables|Default|Get一幀時間) (Variables|Default|Get平滑速度))))